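; Door Blueprint that the player opens and closes with the F key while standing near it.
; An overlap box enables input on entry and disables it on exit.
; Each F press flip-flops between playing and reversing the DoorOpen timeline, gated by a ThirdPersonCharacter cast, which yaws the Door component up to 90 degrees.
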(event OnComponentBeginOverlap(Box)
  (params (OverlappedComponent :type Primitive%20Component%20Object%20Reference) (OtherActor :type Actor%20Object%20Reference) (OtherComp :type Primitive%20Component%20Object%20Reference) (OtherBodyIndex :type Integer) (bFromSweep :type Boolean) (SweepResult :type Hit%20Result%20Structure%20%28by%20ref%29))
  (Input|EnableInput (Game|GetPlayerController 0)))

(event OnComponentEndOverlap(Box)
  (params (OverlappedComponent :type Primitive%20Component%20Object%20Reference) (OtherActor :type Actor%20Object%20Reference) (OtherComp :type Primitive%20Component%20Object%20Reference) (OtherBodyIndex :type Integer))
  (Input|DisableInput (Game|GetPlayerController 0)))

(event Input|KeyboardEvents|F
  (params (Key :type Key%20Structure))
  (:Pressed
    (Utilities|FlowControl|FlipFlop
      (:A
        (Utilities|Casting|CastToThirdPersonCharacter (Game|GetPlayerCharacter 0))
        (bind _opening (Timeline|DoorOpen Play)
          (:Update
            (Transformation|SetRelativeRotation (Variables|Default|GetDoor) (Math|Rotator|MakeRotator 0.0 0.0 (* _opening 9e+01)) false false))))
      (:B
        (Utilities|Casting|CastToThirdPersonCharacter (Game|GetPlayerCharacter 0))
        (Timeline|DoorOpen Reverse)))))

(fn ConstructionScript)
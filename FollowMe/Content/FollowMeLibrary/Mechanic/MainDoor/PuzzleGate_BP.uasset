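; PuzzleGate_BP is a puzzle gate whose door swings open once the collected item count reaches its required maximum.
; OpenDoorCheck compares CurrentItemCollected against MaxItemsCollected and, through a DoOnce, calls OpeningDoor, whose timeline rotates the Door up to 110 degrees in yaw.
; CollectItem is empty and the counter increment sits in disconnected nodes, so this graph never raises the count itself.
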(event Custom|Opening%20Door
  ;[1 1 1] Comment
  (bind _door_anim (Timeline|Open%20Door%20Animation Play)
    (:Update
      (Transformation|SetRelativeRotation (Variables|Default|GetDoor) (Math|Rotator|MakeRotator 0.0 0.0 (* _door_anim 1.1e+02)) false false))))

(event Custom|Collect%20Item
  ;[1 1 1] Comment
)

(event Custom|Open%20Door%20Check
  ;[1 1 1] Comment
  (if (>= (Variables|Default|GetCurrentItemCollected) (Variables|Default|GetMaxItemsCollected))
    (Utilities|FlowControl|DoOnce false
      (:Completed
        (CallFunction|OpeningDoor)))))

(fn ConstructionScript)